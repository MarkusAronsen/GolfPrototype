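; GolfBall_BP is a golf ball character with body, leg and arm meshes that shows a drop shadow and handles dialogue.
; Each tick, a downward sphere trace places the Shadow on the surface below, or hides it when nothing is hit.
; The character's meshes stop receiving decals at BeginPlay.
; PrintDialogue spawns a DialogueBox widget, and Enter advances the first one found if it awaits input.
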(event EventBeginPlay
  (Rendering|SetReceivesDecals (Variables|Default|GetmMesh) false)
  (Rendering|SetReceivesDecals (Variables|Default|GetmLegsMesh) false)
  (Rendering|SetReceivesDecals (Variables|Default|GetmArmsMesh) false))

(event EventPrintDialogue
  (params (displayText :type Array%20of%20Strings))
  (bind _returnvalue (UserInterface|CreateWidget "/Game/GBH/Widgets/UIWidgets/DialogueBox.DialogueBox_C" (Game|GetPlayerController 0)))
  (UserInterface|Viewport|AddtoViewport _returnvalue 0)
  (Variables|/Game/GBH/Widgets/UIWidgets/DialogueBox.DialogueBox_C|SetDialogueText _returnvalue displayText)
  (Default|WidgetInitialized _returnvalue))

(event EventTick
  (params (DeltaSeconds :type Float%20%28single-precision%29))
  (bind _shadow (Variables|Default|GetShadow))
  (bind _mmesh (Variables|Default|GetmMesh))
  (bind _returnvalue (Transformation|GetWorldLocation _mmesh))
  (bind (_outhit _returnvalue_2) (Collision|SphereTraceByChannel _returnvalue (+ _returnvalue "0, 0,-2000.000000") 25.0 "TraceTypeQuery1" false 0 "None"))
  (if _returnvalue_2
    (Rendering|SetVisibility _shadow true false)
    (bind _output_get (Variables|Default|SetDecalTargetLocation (.ImpactPoint (Collision|BreakHitResult _outhit))))
    (Transformation|SetWorldLocation _shadow (.Location (Collision|BreakHitResult _outhit)) false false)
    (Transformation|SetWorldRotation _shadow "90.000000, 0, 0" false false)
    (else
      (Rendering|SetVisibility _shadow false false))))

(event EventSwitchDecalVisibility
  (params (visible :type Boolean))
  (Rendering|SetVisibility (Variables|Default|GetShadow) visible false))

(event Input|KeyboardEvents|Enter
  (params (Key :type Key%20Structure))
  (:Pressed
    (bind _foundwidgets (Widget|GetAllWidgetsOfClass "/Game/GBH/Widgets/UIWidgets/DialogueBox.DialogueBox_C" true))
    (if (> (Utilities|Array|Length _foundwidgets) 0)
      (if (Variables|/Game/GBH/Widgets/UIWidgets/DialogueBox.DialogueBox_C|GetbWaitingForInput (Utilities|Array|Get(acopy) _foundwidgets))
        (Default|NextLine (Utilities|Array|Get(acopy) _foundwidgets))))))

(fn ConstructionScript)