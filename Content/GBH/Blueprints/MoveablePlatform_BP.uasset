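; Moveable platform actor whose Up, Down, Left and Right components glow red, blue, yellow and green respectively to show which direction is pushed.
; The construction script gives each component a dynamic material instance from its colored material.
; Tick polls the four Pushed booleans and switches each matching emission scalar parameter on or off every frame.
; This Blueprint contains no movement logic and never sets those flags itself.
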(event EventBeginPlay)

(event Collision|EventActorBeginOverlap
  (params (OtherActor :type Actor%20Object%20Reference)))

(event EventTick
  (params (DeltaSeconds :type Float%20%28single-precision%29))
  (if (Variables|Default|GetupPushed)
    (Rendering|Material|SetScalarParameterValueonMaterials (Variables|Default|GetUp) "EmissionRed" 3e+01)
    (else
      (Rendering|Material|SetScalarParameterValueonMaterials (Variables|Default|GetUp) "EmissionRed" 0.0)))
  (if (Variables|Default|GetdownPushed)
    (Rendering|Material|SetScalarParameterValueonMaterials (Variables|Default|GetDown) "EmissionBlue" 3e+01)
    (else
      (Rendering|Material|SetScalarParameterValueonMaterials (Variables|Default|GetDown) "EmissionBlue" 0.0)))
  (if (Variables|Default|GetleftPushed)
    (Rendering|Material|SetScalarParameterValueonMaterials (Variables|Default|GetLeft) "EmissionYellow" 3e+01)
    (else
      (Rendering|Material|SetScalarParameterValueonMaterials (Variables|Default|GetLeft) "EmissionYellow" 0.0)))
  (if (Variables|Default|GetrightPushed)
    (Rendering|Material|SetScalarParameterValueonMaterials (Variables|Default|GetRight) "EmissionGreen" 3e+01)
    (else
      (Rendering|Material|SetScalarParameterValueonMaterials (Variables|Default|GetRight) "EmissionGreen" 0.0))))

(fn ConstructionScript
  (Rendering|Material|CreateDynamicMaterialInstance (Variables|Default|GetUp) 0 "/Game/GBH/Materials/Other/MoveablePlatform/RedMoveable_Inst.RedMoveable_Inst" "None" :!class /Script/Engine.PrimitiveComponent)
  (Rendering|Material|CreateDynamicMaterialInstance (Variables|Default|GetDown) 0 "/Game/GBH/Materials/Other/MoveablePlatform/BlueMoveable_Inst.BlueMoveable_Inst" "None" :!class /Script/Engine.PrimitiveComponent)
  (Rendering|Material|CreateDynamicMaterialInstance (Variables|Default|GetLeft) 0 "/Game/GBH/Materials/Other/MoveablePlatform/YellowMoveable_Inst.YellowMoveable_Inst" "None" :!class /Script/Engine.PrimitiveComponent)
  (Rendering|Material|CreateDynamicMaterialInstance (Variables|Default|GetRight) 0 "/Game/GBH/Materials/Other/MoveablePlatform/GreenMoveable_Inst.GreenMoveable_Inst" "None" :!class /Script/Engine.PrimitiveComponent))