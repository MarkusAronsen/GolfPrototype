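; A crumbling block that shakes and shifts color while the player's pawn, matched by object name, overlaps its box.
; Tick drives a sine-based horizontal tremor and ramps the colorAlpha parameter on a dynamic material created in the construction script.
; Leaving reverses the color and snaps the block to its start position unless it is already falling.
; Near-full alpha latches IsFalling; this graph contains no fall movement.
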(event OnComponentBeginOverlap(Box)
  (params (OverlappedComponent :type Primitive%20Component%20Object%20Reference) (OtherActor :type Actor%20Object%20Reference) (OtherComp :type Primitive%20Component%20Object%20Reference) (OtherBodyIndex :type Integer) (bFromSweep :type Boolean) (SweepResult :type Hit%20Result%20Structure%20%28by%20ref%29))
  (if (Utilities|String|Contains (Utilities|GetObjectName OtherActor) (Utilities|GetObjectName (Game|Player|GetPlayerPawn 0)))
    (Variables|Default|SetcolorChanging true)))

(event OnComponentEndOverlap(Box)
  (params (OverlappedComponent :type Primitive%20Component%20Object%20Reference) (OtherActor :type Actor%20Object%20Reference) (OtherComp :type Primitive%20Component%20Object%20Reference) (OtherBodyIndex :type Integer))
  (Variables|Default|SetcolorChanging false))

(event EventBeginPlay
  (Variables|Default|Setoffset (Math|Trig|GetPI))
  (Variables|Default|SetstartPos (Transformation|GetActorLocation)))

(event EventTick
  (params (DeltaSeconds :type Float%20%28single-precision%29))
  (bind _returnvalue (Rendering|Material|GetScalarParameterValue (Variables|Default|GetDynMat) "colorAlpha" :!class /Script/Engine.MaterialInstanceDynamic))
  (if (Variables|Default|GetcolorChanging)
    (Variables|Default|SetcolorChange 1.0)
    (bind _output_get (Variables|Default|Setoffset (+ (Variables|Default|Getoffset) (* (Utilities|Time|GetWorldDeltaSeconds) (Variables|Default|GettremorIntensity)))))
    (if (>= (Variables|Default|Getoffset) (* (Math|Trig|GetPI) 2.0))
      (Variables|Default|Setoffset 0.0))
    (Transformation|AddActorLocalOffset (* (Math|Vector|MakeVector (Math|Trig|Sin(Radians) _output_get) (Math|Trig|Sin(Radians) _output_get) 0.0) 2.0) false false)
    (else
      (Variables|Default|SetcolorChange -1.0)))
  (Rendering|Material|SetScalarParameterValue (Variables|Default|GetDynMat) "colorAlpha" (Math|Float|Clamp(Float) (+ _returnvalue (* (Utilities|Time|GetWorldDeltaSeconds) 1.5 (Variables|Default|GetcolorChange)))) :!class /Script/Engine.MaterialInstanceDynamic)
  (if (> (Math|Float|Clamp(Float) (+ _returnvalue (* (Utilities|Time|GetWorldDeltaSeconds) 1.5 (Variables|Default|GetcolorChange)))) 0.99)
    (Variables|Default|SetbIsFalling true)
    (elif (not (Variables|Default|GetbIsFalling))
      (if (not (Variables|Default|GetcolorChanging))
        (Transformation|SetActorLocation (Variables|Default|GetstartPos) false false)))))

(fn ConstructionScript
  (bind _returnvalue (Rendering|Material|CreateDynamicMaterialInstance (Variables|Default|GetCube) 0 0 "None" :!class /Script/Engine.PrimitiveComponent))
  (Variables|Default|SetDynMat _returnvalue))