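; OscillatingSplineObject is an actor that moves along the spline of a referenced Track actor and draws debug spheres at its position.
; On BeginPlay, a timeline starts at StartPos with a configurable PlayRate, mapping its alpha to distance along the spline to set world location without sweeping.
; Tick independently accumulates time and draws a sphere at a set interval, with configurable size, color and duration.
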(event EventBeginPlay
  (Components|Timeline|SetPlayRate (Variables|Default|Gettimeline0) (Variables|Default|GetplayRate))
  (Components|Timeline|SetNewTime (Variables|Default|Gettimeline0) (Variables|Default|GetstartPos))
  (bind _track (Timeline|timeline0 Play)
    (:Update
      (Variables|Default|SetAlpha _track)
      (Transformation|SetActorLocation (Spline|GetLocationatDistanceAlongSpline (Variables|/Game/GBH/Blueprints/Spline.Spline_C|GetmSpline (Variables|Default|GetTrack)) (Math|Float|Lerp 0.0 (Spline|GetSplineLength (Variables|/Game/GBH/Blueprints/Spline.Spline_C|GetmSpline (Variables|Default|GetTrack))) (Variables|Default|GetAlpha)) "World") false false))))

(event EventTick
  (params (DeltaSeconds :type Float%20%28single-precision%29))
  (bind _output_get (Variables|Default|SetDrawDebugTimer (+ DeltaSeconds (Variables|Default|GetDrawDebugTimer))))
  (if (>= _output_get (Variables|Default|GetDrawDebugInterval))
    (Variables|Default|SetDrawDebugTimer 0.0)
    (Rendering|Debug|DrawDebugSphere (Transformation|GetActorLocation) (Variables|Default|GetDrawDebugSize) (Variables|Default|GetDrawDebugSegments) (Variables|Default|GetDrawDebugColor) (Variables|Default|GetDrawDebugDuration))))

(fn ConstructionScript)