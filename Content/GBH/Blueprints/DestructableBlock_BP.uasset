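; DestructableBlock_BP is a destructible block that shows its remaining health through its material.
; The construction script creates a dynamic material instance on the Cube's first slot and stores it in DestroBlockDynMat.
; Each tick casts self and writes the HitPoints to MaxHitPoints ratio into the HealthColor parameter on the Cube's materials.
; Damage and destruction logic are absent from these graphs.
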(event EventBeginPlay)

(event Collision|EventActorBeginOverlap
  (params (OtherActor :type Actor%20Object%20Reference)))

(event EventTick
  (params (DeltaSeconds :type Float%20%28single-precision%29))
  (bind _asdestructable_block_bp (Utilities|Casting|CastToDestructableBlock_BP self))
  (Rendering|Material|SetScalarParameterValueonMaterials (Variables|Default|GetCube) "HealthColor" (/ (Variables|/Script/Golf04.DestructableBlock|GethitPoints _asdestructable_block_bp) (Variables|/Script/Golf04.DestructableBlock|GetmaxHitPoints _asdestructable_block_bp))))

(fn ConstructionScript
  (bind _returnvalue (Rendering|Material|CreateDynamicMaterialInstance (Variables|Default|GetCube) 0 0 "None" :!class /Script/Engine.PrimitiveComponent))
  (Variables|Default|SetDestroBlockDynMat _returnvalue))