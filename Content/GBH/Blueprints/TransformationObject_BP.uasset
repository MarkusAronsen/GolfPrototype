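; TransformationObject_BP is an actor whose cube gradually changes color while something overlaps its box trigger.
; The construction script creates a dynamic material instance on the cube, and the box's begin and end overlap events toggle a flag.
; Each tick, that flag sets the direction in which the colorAlpha parameter ramps, scaled by delta time and clamped between zero and one.
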(event OnComponentBeginOverlap(Box)
  (params (OverlappedComponent :type Primitive%20Component%20Object%20Reference) (OtherActor :type Actor%20Object%20Reference) (OtherComp :type Primitive%20Component%20Object%20Reference) (OtherBodyIndex :type Integer) (bFromSweep :type Boolean) (SweepResult :type Hit%20Result%20Structure%20%28by%20ref%29))
  (Variables|Default|SetcolorChanging true))

(event OnComponentEndOverlap(Box)
  (params (OverlappedComponent :type Primitive%20Component%20Object%20Reference) (OtherActor :type Actor%20Object%20Reference) (OtherComp :type Primitive%20Component%20Object%20Reference) (OtherBodyIndex :type Integer))
  (Variables|Default|SetcolorChanging false))

(event EventTick
  (params (DeltaSeconds :type Float%20%28single-precision%29))
  (bind _dynamicmaterial (Variables|Default|GetDynamicMaterial))
  (bind _returnvalue (Rendering|Material|GetScalarParameterValue _dynamicmaterial "colorAlpha" :!class /Script/Engine.MaterialInstanceDynamic))
  (if (Variables|Default|GetcolorChanging)
    (Variables|Default|SetcolorChange 1.0)
    (Rendering|Material|SetScalarParameterValue _dynamicmaterial "colorAlpha" (Math|Float|Clamp(Float) (+ _returnvalue (* (Utilities|Time|GetWorldDeltaSeconds) 0.3 (Variables|Default|GetcolorChange)))) :!class /Script/Engine.MaterialInstanceDynamic :!label _label)
    (else
      (Variables|Default|SetcolorChange -1.0)
      (if true
        (goto _label)))))

(fn ConstructionScript
  (bind _returnvalue (Rendering|Material|CreateDynamicMaterialInstance (Variables|Default|GetCube) 0 0 "None" :!class /Script/Engine.PrimitiveComponent))
  (Variables|Default|SetDynamicMaterial _returnvalue))